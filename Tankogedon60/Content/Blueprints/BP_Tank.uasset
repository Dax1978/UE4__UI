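; BP_Tank is a tank Blueprint that creates the player window widget and handles the game-over screen when the tank dies.
; BeginPlay creates and stores W_PlayerWindow if none exists, without adding it to the viewport here.
; Tick polls IsAlive and, when false, pauses the game and adds a new W_EndGame widget to the viewport, with no one-shot guard.
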(event EventBeginPlay
  (Utilities|IsValid (Variables|Default|Getvar_W_PlayerWindow)
    (:Is%20Not%20Valid
      (bind _returnvalue (UserInterface|CreateWidget "/Game/Widgets/W_PlayerWindow.W_PlayerWindow_C" (Game|GetPlayerController 0)))
      (Variables|Default|Setvar_W_PlayerWindow _returnvalue))))

(event Collision|EventActorBeginOverlap
  (params (OtherActor :type Actor%20Object%20Reference)))

(event EventTick
  (params (DeltaSeconds :type Float%20%28single-precision%29))
  (if (not (Variables|Default|GetIsAlive))
    (Game|SetGamePaused true)
    (bind _asplayer_controller (Utilities|Casting|CastToPlayerController (Game|GetPlayerController 0)))
    (bind _returnvalue (UserInterface|CreateWidget "/Game/Widgets/W_EndGame.W_EndGame_C" _asplayer_controller))
    (bind _output_get (Variables|Default|SetEndGameWidget _returnvalue))
    (UserInterface|Viewport|AddtoViewport _output_get 0)))

(fn ConstructionScript)